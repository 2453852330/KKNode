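; BP_Example is an example Blueprint that exercises formatted printing and assorted utility nodes.
; On BeginPlay it stores a random actor from the level as its object value, then calls PrintInfo with variables of many types, an enum converted to string, and a placeholder without an argument.
; Disconnected snippets, which never run, hold PrintText with FormatText, multi-line SaySomething, repeated SayHello calls and a TriGate branching on positive, zero or negative.
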(event `self.ReceiveBeginPlay`
  (bind _outactors (`GameplayStatics.GetAllActorsOfClass` "/Script/Engine.Actor"))
  (set `self.oValue` (`KismetArrayLibrary.Array_Random` _outactors))
  (`|PrintInfo` "int value {a} , float value {b} , str value {c} , bool value {d} , name value {e} , text value {f} , class value {g} , byte value {h} , object value {i}" (`self.iValue`) (`self.fValue`) (`self.sValue`) (`self.bValue`) (`self.nameValue`) (`self.textValue`) (`self.cValue`) (`self.byteValue`) (`self.oValue`))
  (`|PrintInfo` "test enum value {a}" (`|GetEnumeratorNameAsString` (`self.enumValue`)))
  (`|PrintInfo` "枚举 {a}."))

(fn `UserConstructionScript`)