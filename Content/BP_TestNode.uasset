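; BP_TestNode is a test Blueprint for format-string nodes that take named arguments from placeholders in braces.
; On BeginPlay, PrintInfo prints float, string, bool, int and text variables through one format string, which reuses the string placeholder.
; A disconnected TestNode call with arbitrary placeholder names and an unused FormatText node remain in the graph but never run.
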(event `self.ReceiveBeginPlay`
  (`|PrintInfo` "float value : {f} | string value : {a}  | bool value : {b} | int value : {c} | text value : {d} | again string value : {a} | finish " (`self.floatValue`) (`self.stringValue`) (`self.boolValue`) (`self.intValue`) (`self.textValue`)))

(fn `UserConstructionScript`)